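; BP_RandomGenerator is the space shooter's enemy spawner, creating random enemies on a looping timer.
; Each spawn picks among five enemy classes, with the random range widening as the game mode's Level rises.
; It places the enemy at a random one of its scene components tagged "enemyspw".
; SpawnTime drops by half the Level after each spawn, but the timer set at BeginPlay is never reset with it.
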(event `self.ReceiveBeginPlay`
  (`KismetSystemLibrary.K2_SetTimerDelegate` (delegate `Spawn`) (`self.spawnTime`) true)
  (bind _asspace_shooter_ssmode (cast `/Game/00_Space_Shooter/SpaceShooterSSMode` (`GameplayStatics.GetGameMode`)))
  (set `self.As Space Shooter SSMode` _asspace_shooter_ssmode))

(event `Spawn`
  (`self.SpawnEnemy`))

(fn `GetClassToSpawn`
  (params (Max :type Integer))
  (returns (ReturnValue :type "Actor Class Reference"))
  (return (select `int` (`KismetMathLibrary.Clamp` Max 0 4) :`0` "/Game/00_Space_Shooter/Enemies/BP_enemybase.BP_enemybase_C" :`1` "/Game/00_Space_Shooter/Enemies/BP_enemyH.BP_enemyH_C" :`2` "/Game/00_Space_Shooter/Enemies/BP_enemyCrazy.BP_enemyCrazy_C" :`3` "/Game/00_Space_Shooter/Enemies/BP_enemyFreeze.BP_enemyFreeze_C" :`4` "/Game/00_Space_Shooter/Enemies/BP_enemyFollower.BP_enemyFollower_C" :!type "Actor Class Reference")))

(fn `SpawnEnemy`
  (bind _returnvalue (`self.GetComponentsByTag` "/Script/Engine.SceneComponent" "enemyspw"))
  (bind _level (`/Game/00_Space_Shooter/SpaceShooterSSMode.level` (`self.As Space Shooter SSMode`)))
  (bind _returnvalue_2 (`self.GetClassToSpawn` (`KismetMathLibrary.RandomInteger` _level)))
  (`|SpawnActorFromClass` _returnvalue_2 (`SceneComponent.K2_GetComponentToWorld` (`|GetArrayItem` _returnvalue (`KismetMathLibrary.RandomInteger` (`KismetArrayLibrary.Array_Length` _returnvalue)))) "Undefined" "OverrideRootScale" null null)
  (set `self.spawnTime` (- (`self.spawnTime`) (/ _level 2))))

(fn `UserConstructionScript`)