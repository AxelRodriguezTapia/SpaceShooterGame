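; Enemy variant for the space shooter that starts slow and speeds up drastically when shot.
; BeginPlay runs the parent logic, then halves the inherited Speed.
; Overlapping the player damages them and destroys the enemy.
; Player ammo overlaps multiply Speed sharply on each hit and skip the parent's overlap handling, which only runs for other actors.
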(event `self.ReceiveBeginPlay`
  (`parent.ReceiveBeginPlay`)
  (set `self.Speed` (* (`self.Speed`) 0.5)))

(event `self.ReceiveActorBeginOverlap`
  (params (OtherActor :type "Actor Object Reference"))
  (bind _asss_player_caracter (cast `/Game/00_Space_Shooter/Player/SS_PlayerCaracter` OtherActor)
    (:`then`
      (`/Game/00_Space_Shooter/Player/SS_PlayerCaracter.Damage` _asss_player_caracter)
      (`self.K2_DestroyActor`))
    (:`CastFailed`
      (cast `/Game/00_Space_Shooter/Player/Actor_Player_Ammo` OtherActor
        (:`then`
          (set `self.Speed` (* (`self.Speed`) 15.0)))
        (:`CastFailed`
          (`parent.ReceiveActorBeginOverlap` OtherActor))))))

(fn `UserConstructionScript`
  (`parent.UserConstructionScript`))