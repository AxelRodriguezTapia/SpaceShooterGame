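; BP_enemyFollower is a space shooter enemy that homes in on the player and explodes on contact.
; Each Tick it turns to face player character 0 and moves along its stored forward vector at a fixed speed set on BeginPlay, without sweep.
; Overlapping the player calls Damage on it, spawns an Explosion and destroys the enemy.
; The parent Tick is not called, so this movement runs in its place.
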(event `self.ReceiveBeginPlay`
  (`parent.ReceiveBeginPlay`)
  (set `self.Speed` 200.0))

(event `self.ReceiveActorBeginOverlap`
  (params (OtherActor :type "Actor Object Reference"))
  (bind _asss_player_caracter (cast `/Game/00_Space_Shooter/Player/SS_PlayerCaracter` OtherActor)
    (:`then`
      (`/Game/00_Space_Shooter/Player/SS_PlayerCaracter.Damage` _asss_player_caracter)
      (`|SpawnActorFromClass` "/Game/00_Space_Shooter/Effects/Explosion.Explosion_C" (`KismetMathLibrary.Conv_VectorToTransform` (`self.K2_GetActorLocation`)) "Undefined" "MultiplyWithRoot" null null)
      (`self.K2_DestroyActor`))
    (:`CastFailed`
      _))
  (`parent.ReceiveActorBeginOverlap` OtherActor))

(event `self.ReceiveTick`
  (params (DeltaSeconds :type "Float (single-precision)"))
  (`self.K2_SetActorLocation` (+ (`self.K2_GetActorLocation`) (* (* DeltaSeconds (`self.Speed`)) (`self.MovementVector`))))
  (set `self.MovementVector` (`self.GetActorForwardVector`))
  (`self.K2_SetActorRotation` (`KismetMathLibrary.FindLookAtRotation` (`self.K2_GetActorLocation`) (`self.K2_GetActorLocation` (`GameplayStatics.GetPlayerCharacter` 0)))))

(fn `UserConstructionScript`
  (`parent.UserConstructionScript`))