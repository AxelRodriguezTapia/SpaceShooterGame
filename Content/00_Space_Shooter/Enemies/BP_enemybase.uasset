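; Base enemy actor for a space shooter that flies along its initial forward vector and fires enemy bullets from a fire point on a timer.
; Overlap with an actor tagged as player ammo notifies the game mode, plays explosion effects, then after a short delay rolls a random power-up and destroys itself.
; The roll's range exceeds the four power-up options, so some kills drop nothing.
; Overlap with the Tag_BlockInferior tag explodes it without score notification or drop.
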(event `self.ReceiveBeginPlay`
  (set `self.MovementVector` (`self.GetActorForwardVector`))
  (set `self.BulletType` "/Game/00_Space_Shooter/Enemies/enemyBullet.enemyBullet_C"))

(event `self.ReceiveActorBeginOverlap`
  (params (OtherActor :type "Actor Object Reference"))
  (if (`KismetArrayLibrary.Array_Contains` (`Actor.Tags` OtherActor) "ActorPlayerAmoTag")
    (bind _asspace_shooter_ssmode (cast `/Game/00_Space_Shooter/SpaceShooterSSMode` (`GameplayStatics.GetGameMode`)))
    (`/Game/00_Space_Shooter/SpaceShooterSSMode.EnemyDestroyed` _asspace_shooter_ssmode)
    (`GameplayStatics.SpawnEmitterAtLocation` "/Game/StarterContent/Particles/P_Explosion.P_Explosion" (`self.K2_GetActorLocation`))
    (`GameplayStatics.PlaySound2D` "/Game/StarterContent/Audio/Explosion01.Explosion01" 1.0 1.0 0.0 null null)
    (`KismetSystemLibrary.Delay` 0.25)
    (`self.Spawn PowerUp` (`SceneComponent.K2_GetComponentToWorld` (`self.Sphere`)))
    (`self.K2_DestroyActor`)
    (elif (`KismetArrayLibrary.Array_Contains` (`Actor.Tags` OtherActor) "Tag_BlockInferior")
      (`GameplayStatics.SpawnEmitterAtLocation` "/Game/StarterContent/Particles/P_Explosion.P_Explosion" (`self.K2_GetActorLocation`))
      (`GameplayStatics.PlaySound2D` "/Game/StarterContent/Audio/Explosion01.Explosion01" 1.0 1.0 0.0 null null)
      (`KismetSystemLibrary.Delay` 0.25)
      (`self.K2_DestroyActor`))))

(event `self.ReceiveTick`
  (params (DeltaSeconds :type "Float (single-precision)"))
  (bind _currenttime (`self.CurrentTime`))
  (`self.K2_SetActorLocation` (+ (`self.K2_GetActorLocation`) (* (* DeltaSeconds (`self.Speed`)) (`self.MovementVector`))))
  (set `self.CurrentTime` (+ _currenttime DeltaSeconds))
  (if (> _currenttime (`self.DelayShot`))
    (`self.Fire`)
    (set `self.CurrentTime` 0.0)))

(fn `Fire`
  (`|SpawnActorFromClass` (`self.BulletType`) (`SceneComponent.K2_GetComponentToWorld` (`self.FirePoint`)) "Undefined" "MultiplyWithRoot" null null))

(fn `Spawn PowerUp`
  (params (Position :type "Transform Structure"))
  (`|SpawnActorFromClass` (select `int` (`KismetMathLibrary.RandomInteger` 6) :`0` "/Game/00_Space_Shooter/PowerUps/PowerUpFireBoost.PowerUpFireBoost_C" :`1` "/Game/00_Space_Shooter/PowerUps/PowerUpHealth.PowerUpHealth_C" :`2` "/Game/00_Space_Shooter/PowerUps/PowerUpMultyShoot.PowerUpMultyShoot_C" :`3` "/Game/00_Space_Shooter/PowerUps/PowerUpSpeed.PowerUpSpeed_C" :!type "Actor Class Reference") Position "Undefined" "MultiplyWithRoot" null null))

(fn `UserConstructionScript`)